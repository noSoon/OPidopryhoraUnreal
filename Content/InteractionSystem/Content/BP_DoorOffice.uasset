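; BP_DoorOffice is an interactable office door that stays locked until the player picks up the office key.
; On BeginPlay it finds the BP_OfficeKey actor and binds to its OnPick event, which sets Unlocked and then unbinds.
; Interact always fires OnOfficeAttempted, then either toggles a timeline-driven yaw swing of the mesh via FlipFlop or plays a locked-door sound.
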(event `self.ReceiveBeginPlay`
  (`parent.ReceiveBeginPlay`)
  (bind _returnvalue (`GameplayStatics.GetActorOfClass` "/Game/InteractionSystem/Content/BP_OfficeKey.BP_OfficeKey_C"))
  (add `/Game/InteractionSystem/Content/BP_OfficeKey.OnPick` _returnvalue (delegate `Unlock`)))

(event `Unlock`
  (set `self.Unlocked` true)
  (remove `/Game/InteractionSystem/Content/BP_OfficeKey.OnPick` (stale `self.ReceiveBeginPlay` _returnvalue) (delegate `Unlock`)))

(event `/Game/InteractionSystem/Components/BPI_Interaction.Interact`
  (`self.OnOfficeAttempted`)
  (if (`self.Unlocked`)
    (`/Engine/EditorBlueprintResources/StandardMacros.FlipFlop`
      (:`A`
        (bind (_direction _dooropen) (`Timeline|OpenDoorTimeline` :!via `PlayFromStart` :!label _label)
          (:`Update`
            (`SceneComponent.K2_SetRelativeRotation` (`self.StaticMesh`) (`KismetMathLibrary.MakeRotator` 0.0 0.0 (`KismetMathLibrary.Lerp` 0.0 90.0 _dooropen)) false false))))
      (:`B`
        (goto _label :!via `Reverse`)))
    (else
      (`GameplayStatics.PlaySoundAtLocation` "/Game/Sound/Doors/DoorTryLocked_Cue.DoorTryLocked_Cue" (`self.K2_GetActorLocation`) (struct) 1.0 1.0 0.0 null null null null))))

(fn `UserConstructionScript`
  (`parent.UserConstructionScript`))