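; Door Blueprint for the second hall that stays locked until an attempt is made on the office door.
; On BeginPlay it finds BP_DoorOffice and binds to its OnOfficeAttempted dispatcher, which plays a sound, snaps the mesh open, unlocks it, then unbinds.
; Interact plays a locked sound while locked; afterwards a FlipFlop plays or reverses a timeline that lerps mesh yaw, closing first.
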(event `self.ReceiveBeginPlay`
  (`parent.ReceiveBeginPlay`)
  (bind _returnvalue (`GameplayStatics.GetActorOfClass` "/Game/InteractionSystem/Content/BP_DoorOffice.BP_DoorOffice_C"))
  (add `/Game/InteractionSystem/Content/BP_DoorOffice.OnOfficeAttempted` _returnvalue (delegate `UnlockDoor`)))

(event `UnlockDoor`
  (`GameplayStatics.PlaySoundAtLocation` "/Game/Sound/Doors/WoodenDoorOpenClose_Cue.WoodenDoorOpenClose_Cue" (`self.K2_GetActorLocation`) (struct) 1.0 1.0 0.0 null null null null)
  (`SceneComponent.K2_SetRelativeRotation` (`self.StaticMesh`) (`KismetMathLibrary.MakeRotator` 0.0 0.0 90.0) false false)
  (set `self.bUnlocked` true)
  (remove `/Game/InteractionSystem/Content/BP_DoorOffice.OnOfficeAttempted` (stale `self.ReceiveBeginPlay` _returnvalue) (delegate `UnlockDoor`)))

(event `self.Interact`
  (if (`self.bUnlocked`)
    (`/Engine/EditorBlueprintResources/StandardMacros.FlipFlop`
      (:`A`
        (bind (_direction _dooropen) (`Timeline|OpenDoorTimeline` :!via `PlayFromStart` :!label _label)
          (:`Update`
            (`SceneComponent.K2_SetRelativeRotation` (`self.StaticMesh`) (`KismetMathLibrary.MakeRotator` 0.0 0.0 (`KismetMathLibrary.Lerp` 90.0 0.0 _dooropen)) false false))))
      (:`B`
        (goto _label :!via `Reverse`)))
    (else
      (`GameplayStatics.PlaySoundAtLocation` "/Game/Sound/Doors/DoorTryLocked_Cue.DoorTryLocked_Cue" (`self.K2_GetActorLocation`) (struct) 1.0 1.0 0.0 null null null null))))

(fn `UserConstructionScript`
  (`parent.UserConstructionScript`))