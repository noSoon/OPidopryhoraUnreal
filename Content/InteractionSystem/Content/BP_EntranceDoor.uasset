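; BP_EntranceDoor is an interactable entrance door that swings open once.
; On Interact, a Timeline drives the StaticMesh's relative yaw through a Lerp to a quarter turn, and a DoOnce in its update path sets the Opened flag.
; Once Opened is set, further interactions only play a locked-door sound at the actor's location, with no closing logic.
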(event `self.ReceiveBeginPlay`)

(event `/Game/InteractionSystem/Components/BPI_Interaction.Interact`
  (if (`self.Opened`)
    (`GameplayStatics.PlaySoundAtLocation` "/Game/Sound/Doors/DoorTryLocked_Cue.DoorTryLocked_Cue" (`self.K2_GetActorLocation`) (struct) 1.5 1.0 0.0 null null null null)
    (else
      (bind (_direction _dooropen) (`Timeline|Timeline` :!via `PlayFromStart`)
        (:`Update`
          (`SceneComponent.K2_SetRelativeRotation` (`self.StaticMesh`) (`KismetMathLibrary.MakeRotator` 0.0 0.0 (`KismetMathLibrary.Lerp` 0.0 90.0 _dooropen)) false false)
          (`/Engine/EditorBlueprintResources/StandardMacros.DoOnce` false
            (:`Completed`
              (set `self.Opened` true))))))))

(fn `UserConstructionScript`
  (`parent.UserConstructionScript`))