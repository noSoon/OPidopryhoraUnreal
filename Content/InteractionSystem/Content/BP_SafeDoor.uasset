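; An interactable safe door that opens once the player enters the right combination, advancing the game toward its ending transition.
; Interact on a closed safe shows BPW_Safe with UI-only input, and the first attempt fires OnFirstTried after a short delay.
; The widget's OnRightCombination runs OpenDoor, a timeline swinging the mesh open.
; Each timeline update also sets Opened, hides the Widget component and requests the sublevel swap.
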(event `self.ReceiveBeginPlay`)

(event `/Game/InteractionSystem/Components/BPI_Interaction.Interact`
  (bind _returnvalue (`GameplayStatics.GetPlayerController` 0))
  (if (not (`self.Opened`))
    (bind _returnvalue_2 (`|CreateWidget` "/Game/InteractionSystem/Components/BPW_Safe.BPW_Safe_C"))
    (add `/Game/InteractionSystem/Components/BPW_Safe.OnRightCombination` _returnvalue_2 (delegate `OpenDoor`))
    (`UserWidget.AddToViewport` _returnvalue_2 0)
    (`WidgetBlueprintLibrary.SetInputMode_UIOnlyEx` _returnvalue null)
    (set `PlayerController.bShowMouseCursor` true _returnvalue)
    (if (`self.FirstTried`)
      (set `self.FirstTried` false)
      (`KismetSystemLibrary.Delay` 4.0)
      (`self.OnFirstTried`))))

(event `OpenDoor`
  (bind (_direction _dooropen) (`Timeline|Timeline`)
    (:`Update`
      (`SceneComponent.K2_SetRelativeRotation` (`self.StaticMesh`) (`KismetMathLibrary.MakeRotator` 0.0 0.0 (`KismetMathLibrary.Lerp` 0.0 -90.0 _dooropen)) false false)
      (set `self.Opened` true)
      (`SceneComponent.SetHiddenInGame` (`self.Widget`) true false)
      (`GameplayStatics.UnloadStreamLevel` "SubToRemoveExtra")
      (`GameplayStatics.LoadStreamLevel` "SubEndingTransition" true))))

(fn `UserConstructionScript`
  (`parent.UserConstructionScript`))