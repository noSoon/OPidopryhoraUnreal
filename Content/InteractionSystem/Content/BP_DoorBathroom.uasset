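; Bathroom door that stays locked until the player first tries the safe door, playing a locked sound when interacted with before then.
; On BeginPlay it binds Unlock to the BP_SafeDoor's OnFirstTried event.
; Unlock plays a collapse sound, snaps the mesh to a 90-degree yaw and unbinds itself.
; Once unlocked, Interact uses a FlipFlop to play or reverse a timeline that swings the mesh's yaw.
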(event `self.ReceiveBeginPlay`
  (`parent.ReceiveBeginPlay`)
  (bind _returnvalue (`GameplayStatics.GetActorOfClass` "/Game/InteractionSystem/Content/BP_SafeDoor.BP_SafeDoor_C"))
  (add `/Game/InteractionSystem/Content/BP_SafeDoor.OnFirstTried` _returnvalue (delegate `Unlock`)))

(event `Unlock`
  (`GameplayStatics.PlaySoundAtLocation` "/Game/StarterContent/Audio/Collapse_Cue.Collapse_Cue" (`self.K2_GetActorLocation`) (struct) 1.0 1.0 0.0 null null null null)
  (`SceneComponent.K2_SetRelativeRotation` (`self.StaticMesh`) (`KismetMathLibrary.MakeRotator` 0.0 0.0 90.0) false false)
  (set `self.Unlocked` true)
  (remove `/Game/InteractionSystem/Content/BP_SafeDoor.OnFirstTried` (stale `self.ReceiveBeginPlay` _returnvalue) (delegate `Unlock`)))

(event `self.Interact`
  (if (`self.Unlocked`)
    (`/Engine/EditorBlueprintResources/StandardMacros.FlipFlop`
      (:`A`
        (bind (_direction _dooropen) (`Timeline|OpenDoorTimeline` :!via `PlayFromStart` :!label _label)
          (:`Update`
            (`SceneComponent.K2_SetRelativeRotation` (`self.StaticMesh`) (`KismetMathLibrary.MakeRotator` 0.0 0.0 (`KismetMathLibrary.Lerp` 90.0 0.0 _dooropen)) false false))))
      (:`B`
        (goto _label :!via `Reverse`)))
    (else
      (`GameplayStatics.PlaySoundAtLocation` "/Game/Sound/Doors/DoorTryLocked_Cue.DoorTryLocked_Cue" (`self.K2_GetActorLocation`) (struct) 1.0 1.0 0.0 null null null null))))

(fn `UserConstructionScript`
  (`parent.UserConstructionScript`))