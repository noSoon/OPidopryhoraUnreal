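; BP_ObjectLocation is a test actor for the ObjectLocation component's relative-position queries against the player.
; Each tick it passes the first player character's location to IsTargetLeft and prints "Left" or "Right" on screen.
; Disconnected graph snippets also print the direction and angle to the player, but they never run.
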(event `self.ReceiveBeginPlay`)

(event `self.ReceiveTick`
  (params (DeltaSeconds :type "Float (single-precision)"))
  (bind _returnvalue (`ObjectLocation.IsTargetLeft` (`self.ObjectLocation`) (`self.K2_GetActorLocation` (`GameplayStatics.GetPlayerCharacter` 0))))
  (if _returnvalue
    (`KismetSystemLibrary.PrintString` "Left")
    (else
      (`KismetSystemLibrary.PrintString` "Right"))))

(fn `UserConstructionScript`)