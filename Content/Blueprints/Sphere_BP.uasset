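; Sphere_BP is an actor meant to move in a circle in the XY plane at constant height.
; Each Tick advances Angle by Speed times delta time and builds a Cos/Sin offset scaled by Radius.
; The offset is added to the current location rather than a fixed center, so it accumulates per frame and the path's size depends on frame rate.
; The move teleports nothing and skips sweep collision.
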(event `self.ReceiveTick`
  (params (DeltaSeconds :type "Float (single-precision)"))
  (bind _radius (`self.Radius`))
  ;[1 1 1] Рух по колу
  (bind _output_get (set `self.Angle` (+ (* DeltaSeconds (`self.Speed`)) (`self.Angle`))))
  (`self.K2_SetActorLocation` (`KismetMathLibrary.MakeVector` (+ (* (`KismetMathLibrary.Cos` _output_get) _radius) (.x (`self.K2_GetActorLocation`))) (+ (* _radius (`KismetMathLibrary.Sin` _output_get)) (.y (`self.K2_GetActorLocation`))) (.z (`self.K2_GetActorLocation`)))))

(fn `UserConstructionScript`)