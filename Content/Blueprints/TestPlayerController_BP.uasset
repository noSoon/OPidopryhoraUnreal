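; Player controller for a test character that handles movement and a debug-style health input.
; On BeginPlay it casts the controlled pawn to TestCharacter_BP and caches it for the input events.
; The forward and side axes add movement along the character mesh's forward and right vectors, rather than control rotation.
; AddHealthInput calls AddHealth on the character's health component, then GetHealth without using the result.
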(event `self.ReceiveBeginPlay`
  (bind _astest_character_bp (cast `/Game/Blueprints/TestCharacter_BP` (`self.K2_GetPawn`)))
  (set `self.As Test Character BP` _astest_character_bp))

(event `InputAxis|MovingForward`
  (params (AxisValue :type "Float (single-precision)"))
  (bind _as_test_character_bp (`self.As Test Character BP`))
  (`Pawn.AddMovementInput` _as_test_character_bp (`SceneComponent.GetForwardVector` (`Character.Mesh` _as_test_character_bp)) AxisValue false))

(event `InputAxis|MovingSide`
  (params (AxisValue :type "Float (single-precision)"))
  (bind _as_test_character_bp (`self.As Test Character BP`))
  (`Pawn.AddMovementInput` _as_test_character_bp (`SceneComponent.GetRightVector` (`Character.Mesh` _as_test_character_bp)) AxisValue false))

(event `InputAction|AddHealthInput`
  (params (Key :type "Key Structure"))
  (bind _healthcomponent_bp (`/Game/Blueprints/TestCharacter_BP.HealthComponent_BP` (`self.As Test Character BP`)))
  (:`Pressed`
    (`/Game/Blueprints/HealthComponent_BP.AddHealth` _healthcomponent_bp)
    (`/Game/Blueprints/HealthComponent_BP.GetHealth` _healthcomponent_bp)))

(fn `UserConstructionScript`)